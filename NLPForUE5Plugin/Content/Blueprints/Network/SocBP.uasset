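; SocBP is a socket client Blueprint that connects to a local LTP server on BeginPlay.
; It binds connected and message-received events before connecting, with handler functions that leave connection empty and print incoming data to screen.
; Thin wrapper functions expose reconnecting, closing the socket, and sending commands made of a Cmd, Type and Data.
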(event `self.ReceiveBeginPlay`
  (add `self.OnConnected` (`|CreateDelegate` :!event `OnConnectedLTPServer`))
  (add `self.OnRecvMsg` (`|CreateDelegate` :!event `OnRecvMsgFromLTPServer`))
  (`self.ConnetLTP` "127.0.0.1"))

(fn `Close`
  (`self.SocClose`))

(fn `Connect`
  (`self.ConnetLTP` "127.0.0.1"))

(fn `OnConnectedLTPServer`)

(fn `OnRecvMsgFromLTPServer`
  (params (Data :type String))
  (`KismetSystemLibrary.PrintString` Data))

(fn `SendMsgToLTPServer`
  (`self.SendCmd` (`self.Cmd`) (`self.Type`) (`self.Data`)))

(fn `UserConstructionScript`)